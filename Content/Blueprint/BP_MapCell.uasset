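; Maze map cell actor that spawns its own walls and ceiling at BeginPlay, according to five per-side flags.
; Each function derives spawn location and scale from corner and midpoint marker components and the Cube's scale, so pieces follow the cell's size.
; Top, left and right spawn BP_MazeWall; bottom and ceiling show no spawn class, and ceiling prints a debug "Hello".
; The construction script's wall-spawning copy is disconnected.
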(event EventBeginPlay
  (Utilities|FlowControl|Sequence
    (:then_0
      (if (Variables|Default|GetbTopWall)
        (CallFunction|TopWall)))
    (:then_1
      (if (Variables|Default|GetbBottomWall)
        (CallFunction|BottomWall)))
    (:then_2
      (if (Variables|Default|GetbRightWall)
        (CallFunction|RightWall)))
    (:then_3
      (if (Variables|Default|GetbLeftWall)
        (CallFunction|LeftWall)))
    (:then_4
      (if (Variables|Default|GetbCeiling)
        (CallFunction|Ceiling)))))

(fn ConstructionScript)

(fn TopWall
  (bind _midbottom (Variables|Default|GetMidBottom))
  (bind _cube (Variables|Default|GetCube))
  (bind _midtop (Variables|Default|GetMidTop))
  (bind _midtop_2 (Variables|Default|GetMidTop))
  (bind _returnvalue (Transformation|GetWorldLocation _midtop_2))
  (bind _returnvalue_2 (Transformation|GetWorldLocation _midtop))
  (bind _returnvalue_3 (Transformation|GetWorldScale _cube))
  (bind _returnvalue_4 (Transformation|GetWorldLocation _midbottom))
  (bind _returnvalue_5 (- _returnvalue_2 _returnvalue_4))
  (bind _returnvalue_6 (/ (.y _returnvalue_5) 1e+03))
  (Game|SpawnActorfromClass "/Game/Blueprint/BP_MazeWall.BP_MazeWall_C" (Math|Transform|MakeTransform (Math|Vector|MakeVector (.x _returnvalue) (- (.y _returnvalue) (* _returnvalue_6 5e+01)) (- (+ (.z _returnvalue) (* 5e+01 (* (.z _returnvalue_3) 2e+01))) (* (.z _returnvalue_3) 5e+01))) "0, 0, 0" (Math|Vector|MakeVector (/ (.x (- (Transformation|GetWorldLocation (Variables|Default|GetTopRight)) (Transformation|GetWorldLocation (Variables|Default|GetTopLeft)))) 1e+02) _returnvalue_6 (* (.z (Transformation|GetWorldScale (Variables|Default|GetCube))) 2e+01))) "Undefined" "MultiplyWithRoot" 0 0))

(fn BottomWall
  (bind _midtop (Variables|Default|GetMidTop))
  (bind _cube (Variables|Default|GetCube))
  (bind _midbottom (Variables|Default|GetMidBottom))
  (bind _midbottom_2 (Variables|Default|GetMidBottom))
  (bind _returnvalue (Transformation|GetWorldLocation _midbottom_2))
  (bind _returnvalue_2 (Transformation|GetWorldLocation _midbottom))
  (bind _returnvalue_3 (Transformation|GetWorldScale _cube))
  (bind _returnvalue_4 (Transformation|GetWorldLocation _midtop))
  (bind _returnvalue_5 (- _returnvalue_2 _returnvalue_4))
  (bind _returnvalue_6 (/ (.y _returnvalue_5) 1e+03))
  (Game|SpawnActorfromClass "/Game/Blueprint/BP_MazeWall.BP_MazeWall_C" (Math|Transform|MakeTransform (Math|Vector|MakeVector (.x _returnvalue) (- (.y _returnvalue) (* _returnvalue_6 5e+01)) (- (+ (.z _returnvalue) (* 5e+01 (* (.z _returnvalue_3) 2e+01))) (* (.z _returnvalue_3) 5e+01))) "0, 0, 0" (Math|Vector|MakeVector (/ (.x (- (Transformation|GetWorldLocation (Variables|Default|GetBottomRight)) (Transformation|GetWorldLocation (Variables|Default|GetBottomLeft)))) 1e+02) _returnvalue_6 (* (.z (Transformation|GetWorldScale (Variables|Default|GetCube))) 2e+01))) "Undefined" "MultiplyWithRoot" 0 0))

(fn LeftWall
  (bind _topleft (Variables|Default|GetTopLeft))
  (bind _cube (Variables|Default|GetCube))
  (bind _bottomleft (Variables|Default|GetBottomLeft))
  (bind _midleft (Variables|Default|GetMidLeft))
  (bind _returnvalue (Transformation|GetWorldLocation _midleft))
  (bind _returnvalue_2 (Transformation|GetWorldLocation _bottomleft))
  (bind _returnvalue_3 (Transformation|GetWorldScale _cube))
  (bind _returnvalue_4 (Transformation|GetWorldLocation _topleft))
  (bind _returnvalue_5 (- _returnvalue_2 _returnvalue_4))
  (bind _returnvalue_6 (/ (.y _returnvalue_5) 1e+03))
  (Game|SpawnActorfromClass "/Game/Blueprint/BP_MazeWall.BP_MazeWall_C" (Math|Transform|MakeTransform (Math|Vector|MakeVector (.x _returnvalue) (- (.y _returnvalue) (* _returnvalue_6 5e+01)) (- (+ (.z _returnvalue) (* 5e+01 (* (.z _returnvalue_3) 2e+01))) (* (.z _returnvalue_3) 5e+01))) "0, 0, 0" (Math|Vector|MakeVector _returnvalue_6 (/ (.x (- (Transformation|GetWorldLocation (Variables|Default|GetMidLeft)) (Transformation|GetWorldLocation (Variables|Default|GetMidRight)))) 1e+02) (* (.z (Transformation|GetWorldScale (Variables|Default|GetCube))) 2e+01))) "Undefined" "MultiplyWithRoot" 0 0))

(fn RightWall
  (bind _topright (Variables|Default|GetTopRight))
  (bind _cube (Variables|Default|GetCube))
  (bind _bottomright (Variables|Default|GetBottomRight))
  (bind _midright (Variables|Default|GetMidRight))
  (bind _returnvalue (Transformation|GetWorldLocation _midright))
  (bind _returnvalue_2 (Transformation|GetWorldLocation _bottomright))
  (bind _returnvalue_3 (Transformation|GetWorldScale _cube))
  (bind _returnvalue_4 (Transformation|GetWorldLocation _topright))
  (bind _returnvalue_5 (- _returnvalue_2 _returnvalue_4))
  (bind _returnvalue_6 (/ (.y _returnvalue_5) 1e+03))
  (Game|SpawnActorfromClass "/Game/Blueprint/BP_MazeWall.BP_MazeWall_C" (Math|Transform|MakeTransform (Math|Vector|MakeVector (.x _returnvalue) (- (.y _returnvalue) (* _returnvalue_6 5e+01)) (- (+ (.z _returnvalue) (* 5e+01 (* (.z _returnvalue_3) 2e+01))) (* (.z _returnvalue_3) 5e+01))) "0, 0, 0" (Math|Vector|MakeVector _returnvalue_6 (/ (.x (- (Transformation|GetWorldLocation (Variables|Default|GetMidLeft)) (Transformation|GetWorldLocation (Variables|Default|GetMidRight)))) 1e+02) (* (.z (Transformation|GetWorldScale (Variables|Default|GetCube))) 2e+01))) "Undefined" "MultiplyWithRoot" 0 0))

(fn Ceiling
  (bind _mid (Variables|Default|GetMid))
  (bind _returnvalue (Transformation|GetWorldLocation _mid))
  (Development|PrintText "Hello")
  (Game|SpawnActorfromClass "/Game/Blueprint/BP_MazeWall.BP_MazeWall_C" (Math|Transform|MakeTransform (Math|Vector|MakeVector (.x _returnvalue) (.y _returnvalue) (* (.z _returnvalue) 1e+01)) "0, 0, 0" (Transformation|GetWorldScale (Variables|Default|GetCube))) "Undefined" "MultiplyWithRoot" 0 0))