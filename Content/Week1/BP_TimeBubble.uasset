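; BP_TimeBubble is a short-lived actor that slows any actor inside its Bubble component.
; Begin overlap sets the actor's CustomTimeDilation to a tenth of normal and adds it to SlowObjects, while end overlap restores and removes it.
; A one-shot five-second timer calls CleanUp, which loops over SlowObjects, resetting and removing valid entries during iteration, then destroys the bubble.
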(event OnComponentBeginOverlap(Bubble)
  (params (OverlappedComponent :type Primitive%20Component%20Object%20Reference) (OtherActor :type Actor%20Object%20Reference) (OtherComp :type Primitive%20Component%20Object%20Reference) (OtherBodyIndex :type Integer) (bFromSweep :type Boolean) (SweepResult :type Hit%20Result%20Structure%20%28by%20ref%29))
  (Variables|/Script/Engine.Actor|SetCustomTimeDilation OtherActor 0.1)
  (Utilities|Array|Add (Variables|Default|GetSlowObjects) OtherActor))

(event OnComponentEndOverlap(Bubble)
  (params (OverlappedComponent :type Primitive%20Component%20Object%20Reference) (OtherActor :type Actor%20Object%20Reference) (OtherComp :type Primitive%20Component%20Object%20Reference) (OtherBodyIndex :type Integer))
  (Variables|/Script/Engine.Actor|SetCustomTimeDilation OtherActor 1.0)
  (Utilities|Array|RemoveItem (Variables|Default|GetSlowObjects) OtherActor))

(event Custom|CleanUp
  (for _array_element (Variables|Default|GetSlowObjects)
    (Utilities|IsValid _array_element
      (:Is%20Valid
        (Variables|/Script/Engine.Actor|SetCustomTimeDilation _array_element 1.0)
        (Utilities|Array|RemoveItem (Variables|Default|GetSlowObjects) _array_element))))
  (Actor|DestroyActor))

(event EventBeginPlay
  (Utilities|Time|SetTimerbyEvent (delegate Custom|CleanUp) 5.0))

(fn ConstructionScript)