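; BP_Gold is an interactable gold pickup that rolls a random value and displays it on a text render.
; The construction script chains CreateMesh threshold checks, each running only after the previous passes, so only top-tier values get meshes, three with randomized offset and scale.
; BeginPlay caches BP_ThirdPersonGameMode and sets the text.
; Interract adds the value to the game mode's PlayerGold, prints the total and destroys the actor.
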(event EventBeginPlay
  (bind _asbp_third_person_game_mode (Utilities|Casting|CastToBP_ThirdPersonGameMode (Game|GetGameMode)))
  (Variables|Default|SetGameMode _asbp_third_person_game_mode)
  (Rendering|Components|TextRender|SetText (Variables|Default|GetTextRender) (Utilities|Text|ToText(Integer) (Variables|Default|GetItemGold))))

(event EventInterract
  (bind _gamemode (Variables|Default|GetGameMode))
  (bind _output_get (Variables|/Game/ThirdPerson/Blueprints/BP_ThirdPersonGameMode.BP_ThirdPersonGameMode_C|SetPlayerGold _gamemode (+ (Variables|/Game/ThirdPerson/Blueprints/BP_ThirdPersonGameMode.BP_ThirdPersonGameMode_C|GetPlayerGold _gamemode) (Variables|Default|GetItemGold))))
  (Development|PrintString (Utilities|String|Append "Current Gold" (Utilities|String|ToString(Integer) _output_get)))
  (Actor|DestroyActor))

(fn ConstructionScript
  (Variables|Default|SetItemGold (Math|Random|RandomIntegerinRange 1 99))
  (Utilities|CreateMesh (>= (Variables|Default|GetItemGold) 76)
    (:then
      (Utilities|CreateMesh (>= (Variables|Default|GetItemGold) 26)
        (:then
          (Utilities|CreateMesh (>= (Variables|Default|GetItemGold) 1)))))))