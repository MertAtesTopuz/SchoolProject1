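; BP_MazeCell is a modular maze cell actor that builds one square tile with optional walls, ceiling and light.
; Its Construction Script scales the floor from GridSize, derives wall thickness from it, and adds a mesh for each enabled wall or ceiling flag.
; SizeToCubeScale supplies mesh scales from cell dimensions.
; A centered point light near the top is added with configurable color when intensity is above zero.
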(event EventBeginPlay)

(event Collision|EventActorBeginOverlap
  (params (OtherActor :type Actor%20Object%20Reference)))

(event EventTick
  (params (DeltaSeconds :type Float%20%28single-precision%29)))

(fn ConstructionScript
  (bind _gridsize (Variables|Default|GetGridSize))
  (LocalVariables|SetWallLength _gridsize)
  (LocalVariables|SetWallThicness (* _gridsize 0.1))
  (Transformation|SetRelativeScale3D (Variables|Default|GetFloor) (Utilities|SizetoCubeScale (Math|Vector|MakeVector (LocalVariables|GetWallLength) (LocalVariables|GetWallLength) (LocalVariables|GetWallThicness))))
  (Utilities|FlowControl|Sequence
    (:then_0
      (if (Variables|Default|GetWestWall)
        (AddComponent|AddStaticMeshComponent false (Math|Transform|MakeTransform "0, 0, 0" "0, 0, 0" (Utilities|SizetoCubeScale (Math|Vector|MakeVector (LocalVariables|GetWallLength) (LocalVariables|GetWallThicness) (Variables|Default|GetWallHeight)))))))
    (:then_1
      (if (Variables|Default|GetSouthWall)
        (AddComponent|AddStaticMeshComponent false (Math|Transform|MakeTransform "0, 0, 0" "0, 0, 0" (Utilities|SizetoCubeScale (Math|Vector|MakeVector (LocalVariables|GetWallThicness) (LocalVariables|GetWallLength) (Variables|Default|GetWallHeight)))))))
    (:then_2
      (if (Variables|Default|GetNorthWall)
        (AddComponent|AddStaticMeshComponent false (Math|Transform|MakeTransform (Math|Vector|MakeVector (- (LocalVariables|GetWallLength) (LocalVariables|GetWallThicness)) 0.0 0.0) "0, 0, 0" (Utilities|SizetoCubeScale (Math|Vector|MakeVector (LocalVariables|GetWallThicness) (LocalVariables|GetWallLength) (Variables|Default|GetWallHeight)))))))
    (:then_3
      (if (Variables|Default|GetEastWall)
        (AddComponent|AddStaticMeshComponent false (Math|Transform|MakeTransform (Math|Vector|MakeVector 0.0 (- (LocalVariables|GetWallLength) (LocalVariables|GetWallThicness)) 0.0) "0, 0, 0" (Utilities|SizetoCubeScale (Math|Vector|MakeVector (LocalVariables|GetWallLength) (LocalVariables|GetWallThicness) (Variables|Default|GetWallHeight)))))))
    (:then_4
      (if (Variables|Default|GetCeiling)
        (AddComponent|AddStaticMeshComponent false (Math|Transform|MakeTransform (Math|Vector|MakeVector 0.0 0.0 (Variables|Default|GetWallHeight)) "0, 0, 0" (Utilities|SizetoCubeScale (Math|Vector|MakeVector (LocalVariables|GetWallLength) (LocalVariables|GetWallLength) (LocalVariables|GetWallThicness)))))))
    (:then_5
      (if (> (Variables|Default|GetLightIntencity) 0.0)
        (bind _returnvalue (AddComponent|AddPointLightComponent false (Math|Transform|MakeTransform (Math|Vector|MakeVector (* (LocalVariables|GetWallLength) 0.5) (* (LocalVariables|GetWallLength) 0.5) (* (Variables|Default|GetWallHeight) 0.9)) "0, 0, 0" "1.000000,1.000000,1.000000")))
        (bind _output_get (Variables|Default|SetLightComp _returnvalue))
        (Rendering|Components|Light|SetLightColor _output_get (Variables|Default|GetLightColor) true)
        (Rendering|Components|Light|SetIntensity _output_get (Variables|Default|GetLightIntencity))))))