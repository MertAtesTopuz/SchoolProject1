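; BP_SpikeTrap is a spike trap actor that hurts the player on contact and can be permanently disabled by an event from the player character.
; Overlapping the activation volume plays a timeline that moves the spike vertically, while overlapping the damage box reduces the player's health.
; It binds to the character's trap event at BeginPlay; a matching TrapType lowers the spike, turns off damage collision and destroys the timeline component to block reactivation.
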(event OnComponentBeginOverlap(DamageBox)
  (params (OverlappedComponent :type Primitive%20Component%20Object%20Reference) (OtherActor :type Actor%20Object%20Reference) (OtherComp :type Primitive%20Component%20Object%20Reference) (OtherBodyIndex :type Integer) (bFromSweep :type Boolean) (SweepResult :type Hit%20Result%20Structure%20%28by%20ref%29))
  (if (== OtherActor (Variables|Default|GetCharacter))
    (Default|HealthUpadate (Variables|Default|GetCharacter) -15.0)))

(event OnComponentBeginOverlap(ActivateCol)
  (params (OverlappedComponent :type Primitive%20Component%20Object%20Reference) (OtherActor :type Actor%20Object%20Reference) (OtherComp :type Primitive%20Component%20Object%20Reference) (OtherBodyIndex :type Integer) (bFromSweep :type Boolean) (SweepResult :type Hit%20Result%20Structure%20%28by%20ref%29))
  (if (== OtherActor (Variables|Default|GetCharacter))
    (Variables|Default|GetSpikeTL
      (:then
        (bind _newtrack_0 (Timeline|SpikeTL PlayFromStart)
          (:Update
            (Transformation|SetRelativeLocation (Variables|Default|GetSpike) (Math|Vector|MakeVector 0.0 0.0 _newtrack_0) false false))))
      (:else))))

(event Custom|DPTrapEvent
  (params (TrapType :type E_TrapTypes%20Enum :default "NewEnumerator0"))
  (if (Utilities|Enum|Equal(Enum) TrapType (Variables|Default|GetTrapType))
    (Transformation|SetRelativeLocation (Variables|Default|GetSpike) "0.000000,0.000000,-275.000000" false false)
    (Collision|SetCollisionEnabled (Variables|Default|GetDamageBox) "NoCollision")
    (Components|DestroyComponent (Variables|Default|GetSpikeTL))))

(event EventBeginPlay
  (bind _asbp_third_person_character (Utilities|Casting|CastToBP_ThirdPersonCharacter (Game|GetPlayerCharacter 0)))
  (bind _output_get (Variables|Default|SetCharacter _asbp_third_person_character))
  (EventDispatchers|BindEventtoDPTrap _output_get (delegate Custom|DPTrapEvent)))

(fn ConstructionScript)