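; BP_Keys is an interactable key pickup that hands its key number to the game mode.
; The construction script colors the sphere red or green from KeyNumber.
; On Interract, it overwrites the Keys value on the BP_ThirdPersonGameMode cached at BeginPlay, prints the acquired key's name and destroys itself.
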(event EventBeginPlay
  (bind _asbp_third_person_game_mode (Utilities|Casting|CastToBP_ThirdPersonGameMode (Game|GetGameMode)))
  (Variables|Referances|SetGameMode _asbp_third_person_game_mode))

(event EventInterract
  (bind _output_get (Variables|/Game/ThirdPerson/Blueprints/BP_ThirdPersonGameMode.BP_ThirdPersonGameMode_C|SetKeys (Variables|Referances|GetGameMode) (Variables|Default|GetKeyNumber)))
  (Development|PrintString (Utilities|String|Append "key " (Utilities|Array|Get(acopy) (Variables|Default|GetNames) _output_get) " acquired"))
  (Actor|DestroyActor))

(fn ConstructionScript
  (bind _sphere (Variables|Default|GetSphere))
  (switch int (Variables|Default|GetKeyNumber)
    (:0
      (Rendering|Material|SetMaterial _sphere 0 "/Game/Materials/M_Red.M_Red"))
    (:1
      (Rendering|Material|SetMaterial _sphere 0 "/Game/Materials/M_Green.M_Green"))))