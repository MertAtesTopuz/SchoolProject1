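; BP_Door is a locked door actor that swings open when interacted with while the player holds the matching key.
; On BeginPlay it caches the third-person game mode, and Interract compares that game mode's Keys value to the door's KeyNumber.
; A match plays a timeline that lerps the MiddlePoint pivot's rotation; otherwise it prints a wrong-key message.
; The construction script colors the cube red or green from KeyNumber.
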(event EventBeginPlay
  (bind _asbp_third_person_game_mode (Utilities|Casting|CastToBP_ThirdPersonGameMode (Game|GetGameMode)))
  (Variables|Default|SetGameMode _asbp_third_person_game_mode))

(event EventInterract
  (if (== (Variables|/Game/ThirdPerson/Blueprints/BP_ThirdPersonGameMode.BP_ThirdPersonGameMode_C|GetKeys (Variables|Default|GetGameMode)) (Variables|Default|GetKeyNumber))
    (bind _newtrack_0 (Timeline|Door_Rotate Play)
      (:Update
        (Transformation|SetRelativeRotation (Variables|Default|GetMiddlePoint) (Math|Rotator|Lerp(Rotator) (Variables|Default|GetStartLocation) (Variables|Default|GetFinishLocation) _newtrack_0) false false)))
    (else
      (Development|PrintString "You dont have the correct key"))))

(fn ConstructionScript
  (bind _cube (Variables|Default|GetCube))
  (switch int (Variables|Default|GetKeyNumber)
    (:0
      (Rendering|Material|SetMaterial _cube 0 "/Game/Materials/M_Red.M_Red"))
    (:1
      (Rendering|Material|SetMaterial _cube 0 "/Game/Materials/M_Green.M_Green"))))