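; BP_Switch is an interactable switch tied to one trap type, apparently used to turn off traps of that type.
; On BeginPlay it caches the player's BP_ThirdPersonCharacter and shows its trap type enum on a text render label.
; Interacting passes that enum to the character's CallDPTrap and prints a "Turn Off Traps" message, so the switch holds no direct references to traps.
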(event EventBeginPlay
  (bind _asbp_third_person_character (Utilities|Casting|CastToBP_ThirdPersonCharacter (Game|GetPlayerCharacter 0)))
  (Variables|Default|SetCharacter _asbp_third_person_character)
  (Rendering|Components|TextRender|SetText (Variables|Default|GetTextRender) (Utilities|Text|ToText(String) (Utilities|String|EnumtoString (Variables|Default|GetTrapTypeEnum)))))

(event EventInterract
  (Default|CallDPTrap (Variables|Default|GetCharacter) (Variables|Default|GetTrapTypeEnum))
  (Development|PrintString "Turn Off Traps"))

(fn ConstructionScript)